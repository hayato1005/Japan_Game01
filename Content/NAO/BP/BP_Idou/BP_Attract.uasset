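; BP_Attract is an actor that pulls itself toward the goal point in the level when the P key is pressed.
; It enables player input on BeginPlay, then on key press finds the first BP_GoalPoint and stores its current location as the start.
; A timeline drives a lerp from that start to the goal's live location, moving the actor with swept collision.
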(event EventBeginPlay
  ;[1 1 1] インプットキーを有効化
  (Input|EnableInput (Game|GetPlayerController 0)))

(event Collision|EventActorBeginOverlap
  (params (OtherActor :type Actor%20Object%20Reference)))

(event EventTick
  (params (DeltaSeconds :type Float%20%28single-precision%29)))

(event Input|KeyboardEvents|P
  (params (Key :type Key%20Structure :default "None"))
  (:Pressed
    ;[1 1 1] BP_GoalPointの座標を取得
    (bind _outactors (Actor|GetAllActorsOfClass "/Game/NAO/BP/BP_Idou/BP_GoalPoint.BP_GoalPoint_C"))
    (Variables|Default|SetGoalPoint (Utilities|Array|Get(acopy) _outactors))
    (Variables|Default|SetStartLocation (Transformation|GetActorLocation))
    (bind _新規track_1 (Timeline|タイムライン_0 PlayFromStart)
      (:Update
        (Transformation|SetActorLocation (Math|Vector|Lerp(Vector) (Variables|Default|GetStartLocation) (Transformation|GetActorLocation (Variables|Default|GetGoalPoint)) _新規track_1) true false)))))

(fn ConstructionScript)