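; Wire actor with a cable and projectile movement that the side-scroller player hangs from after touching its tip Box.
; While the character's Grab is false, a one-time step attaches the cable, enables capsule physics and constrains the capsule to the Cube.
; When Grab is true, Tick undoes this and interpolates the character back to its stored rotation, then clears the contact.
; A Hit component collision stops the projectile and destroys the actor shortly after.
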(event OnComponentBeginOverlap(Box)
  (params (OverlappedComponent :type Primitive%20Component%20Object%20Reference) (OtherActor :type Actor%20Object%20Reference) (OtherComp :type Primitive%20Component%20Object%20Reference) (OtherBodyIndex :type Integer) (bFromSweep :type Boolean) (SweepResult :type Hit%20Result%20Structure%20%28by%20ref%29))
  ;[1 1 1] Boxにキャラクターが触れたらTure
  (Utilities|Casting|CastToSideScrollerCharacter OtherActor)
  (Variables|Default|SetBox%20In true))

(event OnComponentHit(Hit)
  (params (HitComponent :type Primitive%20Component%20Object%20Reference) (OtherActor :type Actor%20Object%20Reference) (OtherComp :type Primitive%20Component%20Object%20Reference) (NormalImpulse :type Vector :default "0, 0, 0") (Hit :type Hit%20Result%20Structure%20%28by%20ref%29))
  ;[1 1 1] 物に当たると止まって（　）秒後に消える
  (Development|PrintString "Hit")
  (Components|Movement|StopMovementImmediately (Variables|Default|GetProjectileMovement))
  (Utilities|FlowControl|Delay 0.5)
  (Actor|DestroyActor))

(event EventBeginPlay)

(event Collision|EventActorBeginOverlap
  (params (OtherActor :type Actor%20Object%20Reference)))

(event EventTick
  (params (DeltaSeconds :type Float%20%28single-precision%29))
  (bind _cable (Variables|Default|GetCable))
  (bind _physicsconstraint (Variables|Default|GetPhysicsConstraint))
  (bind _cube (Variables|Default|GetCube))
  ;[1 1 1] ワイヤーの先端(Box)に当たったら
  (if (Variables|Default|GetBox%20In)
    (bind _asside_scroller_character (Utilities|Casting|CastToSideScrollerCharacter (Game|GetPlayerCharacter 0)))
    (Utilities|FlowControl|Sequence
      (:then_0
        (if (Variables|/Game/SideScrollerBP/Blueprints/SideScrollerCharacter.SideScrollerCharacter_C|GetGrab _asside_scroller_character)
          (Class|CableComponent|SetAttachEndto _cable 0 "None" "None")
          (Physics|SetSimulatePhysics (Variables|/Script/Engine.Character|GetCapsuleComponent _asside_scroller_character) false)
          (Class|PhysicsConstraintComponent|SetConstrainedComponents _physicsconstraint _cube "None" (Variables|Default|GetSphere) "None")
          (Variables|Default|SetRotationCharctor true)
          (else
            (Utilities|FlowControl|DoOnce false
              (:Completed
                (Class|CableComponent|SetAttachEndto _cable _asside_scroller_character "None" "None")
                (Physics|SetSimulatePhysics (Variables|/Script/Engine.Character|GetCapsuleComponent _asside_scroller_character) true)
                (Class|PhysicsConstraintComponent|SetConstrainedComponents _physicsconstraint _cube "None" (Variables|/Script/Engine.Character|GetCapsuleComponent _asside_scroller_character) "None"))))))
      (:then_1
        ;[1 1 1] Rotationが１？になったらワイヤーから離れる？
        (if (Variables|Default|GetRotationCharctor)
          (Transformation|SetActorRotation _asside_scroller_character (Math|Interpolation|RInterpTo (Transformation|GetActorRotation _asside_scroller_character) (Variables|/Game/SideScrollerBP/Blueprints/SideScrollerCharacter.SideScrollerCharacter_C|GetRotation _asside_scroller_character) 0.0 1e+01))
          (if (Math|Rotator|Equal(Rotator) (Transformation|GetActorRotation _asside_scroller_character) (Variables|/Game/SideScrollerBP/Blueprints/SideScrollerCharacter.SideScrollerCharacter_C|GetRotation _asside_scroller_character) 1.0)
            (Variables|Default|SetRotationCharctor false)
            (Variables|Default|SetBox%20In false)))))))

(fn ConstructionScript)